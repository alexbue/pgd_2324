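; Actor component that launches a one-time visual novel dialogue when the player pawn overlaps its owning actor.
; On BeginPlay it binds to the owner's overlap events and creates a start-dialog prompt widget, which is stored but never displayed.
; The first player overlap disables pawn input, shows UWG_Dialogue, calls its begin event and destroys the component.
; The end-overlap handler is empty.
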(event Custom|ActorEndOverlap
  (params (OverlappedActor :type Actor%20Object%20Reference) (OtherActor :type Actor%20Object%20Reference)))

(event Custom|ActorBeginOverlap
  (params (OverlappedActor :type Actor%20Object%20Reference) (OtherActor :type Actor%20Object%20Reference))
  (bind _returnvalue (Game|Player|GetPlayerPawn 0))
  ;[1 1 1] Launch Dialogue
  (if (== OtherActor _returnvalue)
    (Utilities|FlowControl|DoOnce false
      (:Completed
        (bind _returnvalue_2 (UserInterface|CreateWidget "/Game/VisualNovel/Blueprints/Widgets/UWG_Dialogue.UWG_Dialogue_C"))
        (Input|DisableInput _returnvalue (Game|GetPlayerController 0))
        (bind _output_get (Variables|Default|SetDialogue_Widget _returnvalue_2))
        (UserInterface|Viewport|AddtoViewport _output_get 0)
        (bind _asuwg_dialogue (Utilities|Casting|CastToUWG_Dialogue _output_get))
        (Default|BeginDialogueEvent _asuwg_dialogue)
        (Components|DestroyComponent)))))

(event EventBeginPlay
  ;[1 1 1] Bind to Begin Overlap
  (bind _asactor (Utilities|Casting|CastToActor (Utilities|GetOuterObject self)))
  (Collision|BindEventtoOnActorBeginOverlap _asactor (delegate Custom|ActorBeginOverlap))
  (Collision|BindEventtoOnActorEndOverlap _asactor (delegate Custom|ActorEndOverlap))
  ;[1 1 1] Draw Dialog Activate Button
  (bind _returnvalue (UserInterface|CreateWidget "/Game/VisualNovel/Blueprints/Widgets/UWG_StartDialog.UWG_StartDialog_C" (Game|GetPlayerController 0)))
  (Variables|Default|SetNewVar _returnvalue))

(event EventTick
  (params (DeltaSeconds :type Float%20%28single-precision%29)))