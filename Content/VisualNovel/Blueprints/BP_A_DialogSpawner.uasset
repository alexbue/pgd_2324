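; Visual novel trigger actor that spawns a dialogue widget when the player interacts with it or enters its box, depending on DialogueSpawnerMode.
; Manual mode registers the actor as the player's InteractionActor during overlap and brightens a prompt widget, while On Overlap plays once and destroys the actor.
; PlaybackDialogue creates UWG_Dialogue and begins it, and SkipDialogueLine flags that widget to skip to end.
; Immediate and Disabled only hide the prompt here.
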(event OnComponentBeginOverlap(Box)
  (params (OverlappedComponent :type Primitive%20Component%20Object%20Reference) (OtherActor :type Actor%20Object%20Reference) (OtherComp :type Primitive%20Component%20Object%20Reference) (OtherBodyIndex :type Integer) (bFromSweep :type Boolean) (SweepResult :type Hit%20Result%20Structure%20%28by%20ref%29))
  ;[1 1 1] On Overlap Begin
  (if (== OtherActor (Game|Player|GetPlayerPawn 0))
    (switch Utilities|FlowControl|Switch|SwitchonDialogSpawnerMode (Variables|Default|GetDialogueSpawnerMode)
      (:NewEnumerator1
        (Variables|Default|SetInteractionPossible? true)
        (Widget|SetRenderOpacity (UserInterface|GetWidget (Variables|Default|GetWidget_Manual)) 1.0)
        (bind _asplayer (Utilities|Casting|CastToPlayer OtherActor))
        (Variables|/Game/Player/Player.Player_C|SetInteractionActor _asplayer self))
      (:NewEnumerator0
        (Utilities|PlaybackDialogue)
        (Actor|DestroyActor)))))

(event OnComponentEndOverlap(Box)
  (params (OverlappedComponent :type Primitive%20Component%20Object%20Reference) (OtherActor :type Actor%20Object%20Reference) (OtherComp :type Primitive%20Component%20Object%20Reference) (OtherBodyIndex :type Integer))
  ;[1 0.2289 0.1292] On Overlap End
  (if (and (Utilities|Enum|Equal(Enum) (Variables|Default|GetDialogueSpawnerMode) "NewEnumerator1") (== OtherActor (Game|Player|GetPlayerPawn 0)))
    (Variables|Default|SetInteractionPossible? false)
    (Widget|SetRenderOpacity (UserInterface|GetWidget (Variables|Default|GetWidget_Manual)) 0.5)
    (bind _asplayer (Utilities|Casting|CastToPlayer OtherActor))
    (Variables|/Game/Player/Player.Player_C|SetInteractionActor _asplayer 0)))

(event EventInteract
  (bind _widget_manual (Variables|Default|GetWidget_Manual))
  (bind _returnvalue (UserInterface|GetWidget _widget_manual))
  (bind _renderopacity (Variables|/Script/UMG.Widget|GetRenderOpacity _returnvalue))
  ;[0.2464 0.3785 1] Auto Play Dialogue
  (Utilities|FlowControl|DoOnce false :!label _label
    (:Completed
      (Variables|Default|SetWidget%20Render%20Opacity%20TMP _renderopacity)
      (Widget|SetRenderOpacity _returnvalue 0.0)
      (Utilities|PlaybackDialogue)
      (Widget|SetRenderOpacity (UserInterface|GetWidget (Variables|Default|GetWidget_Manual)) _renderopacity)
      (goto _label Reset))))

(event EventSkipDialogueLine
  (bind _dialogue_widget (Variables|Default|GetDialogue_Widget))
  (if (Utilities|IsValid _dialogue_widget)
    (bind _asuwg_dialogue (Utilities|Casting|CastToUWG_Dialogue _dialogue_widget))
    (Variables|/Game/VisualNovel/Blueprints/Widgets/UWG_Dialogue.UWG_Dialogue_C|SetSkip%20to%20end _asuwg_dialogue true)))

(event EventBeginPlay
  (bind _widget_manual (Variables|Default|GetWidget_Manual))
  (bind _returnvalue (UserInterface|GetWidget _widget_manual))
  ;[1 1 1] BEGIN PLAY
  (switch Utilities|FlowControl|Switch|SwitchonDialogSpawnerMode (Variables|Default|GetDialogueSpawnerMode)
    (:NewEnumerator1
      (Widget|SetRenderOpacity _returnvalue 0.5))
    (:NewEnumerator0
      (Components|Activation|SetActive _widget_manual false false :!label _label)
      (Widget|SetRenderOpacity _returnvalue 0.0))
    (:NewEnumerator2
      (goto _label))
    (:NewEnumerator3
      (goto _label))))

(fn ConstructionScript)